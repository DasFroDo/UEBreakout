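; Player pawn for a Breakout-style game that slides a paddle mesh sideways within clamped limits and quits on Escape.
; Device tilt, scaled by an intensity, moves the paddle, then stores its Y position to yaw the camera arm root in the opposite direction.
; Mouse X moves the paddle directly over a wider range without updating the yaw.
; The Hit handler for ball impulse is an unfinished stub.
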(event `InputVectorAxis|Tilt`
  (params (AxisValue :type "Vector Structure"))
  ;[0 1 0.0375] Android Controls
  (`self.UpdatePaddlePosition` AxisValue)
  ;;[1 1 1] Write Paddle Y Location to Variable (might be needed later)
  (set `self.PaddleLocationY` (.y (`SceneComponent.RelativeLocation` (`self.StaticMesh`))))
  (`self.UpdateCameraYaw`))

(event `Key|Escape`
  (params (Key :type "Key Structure" :default "AnyKey"))
  ;[0 0.3457 1] PC Controls
  (:`Pressed`
    (`KismetSystemLibrary.QuitGame` null "Quit")))

(event `InputAxisKey|MouseX`
  (params (AxisValue :type "Float (single-precision)"))
  ;[0 0.3457 1] PC Controls
  (`SceneComponent.K2_SetRelativeLocation` (`self.StaticMesh`) (`KismetMathLibrary.MakeVector` (.x (`SceneComponent.RelativeLocation` (`self.StaticMesh`))) (`KismetMathLibrary.FClamp` (+ AxisValue (.y (`SceneComponent.RelativeLocation` (`self.StaticMesh`)))) -100.0 100.0) (.z (`SceneComponent.RelativeLocation` (`self.StaticMesh`)))) false false))

(event `self.ReceiveHit`
  (params (MyComp :type "PrimitiveComponent Object Reference") (Other :type "Actor Object Reference") (OtherComp :type "PrimitiveComponent Object Reference") (bSelfMoved :type Boolean) (HitLocation :type "Vector Structure") (HitNormal :type "Vector Structure") (NormalImpulse :type "Vector Structure") (Hit :type "HitResult Structure (by ref)"))
  (bind (_bblockinghit _binitialoverlap _time _location _impactpoint _normal _impactnormal _physmat _hitactor) (`GameplayStatics.BreakHitResult` Hit))
  ;[1 1 1] Calculate Ingoing to Outgoing Impulse
  (if (!= (`GameplayStatics.GetObjectClass` _hitactor) (`self.GameBall`))
    (cast `/Game/Blueprints/GameBall` _hitactor)))

(fn `UpdateCameraYaw`
  (`SceneComponent.K2_SetRelativeRotation` (`self.Arm Root`) (`KismetMathLibrary.MakeRotator` 0.0 0.0 (/ (`self.PaddleLocationY`) -10.0)) false false))

(fn `UpdatePaddlePosition`
  (params (InVec :type "Vector Structure"))
  (`SceneComponent.K2_SetRelativeLocation` (`self.StaticMesh`) (`KismetMathLibrary.MakeVector` (.x (`SceneComponent.RelativeLocation` (`self.StaticMesh`))) (`KismetMathLibrary.FClamp` (+ (* (.x InVec) (`self.TiltIntensity`)) (.y (`SceneComponent.RelativeLocation` (`self.StaticMesh`)))) -50.0 50.0) (.z (`SceneComponent.RelativeLocation` (`self.StaticMesh`)))) false false))

(fn `UserConstructionScript`)