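; GameBall is a physics-driven ball that launches itself along the world Z axis shortly after spawning.
; BeginPlay waits briefly, then applies InitialVelocity as a velocity-change impulse, which ignores mass.
; Tick caches the ball's linear velocity in CurrentVelocity.
; ApplyImpactImpulse is unfinished: it only prints the outgoing normal, and its AddImpulse node is unconnected.
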(event `self.ReceiveBeginPlay`
  ;[1 1 1] Start Ball on Spawn
  (`KismetSystemLibrary.Delay` 1.0)
  (`PrimitiveComponent.AddImpulse` (`self.Ball`) (`KismetMathLibrary.MakeVector` 0.0 0.0 (`self.InitialVelocity`)) "None" true))

(event `self.ReceiveTick`
  (params (DeltaSeconds :type "Float (single-precision)"))
  ;[1 1 1] Write current Velocity to Variable
  (bind _returnvalue (`PrimitiveComponent.GetPhysicsLinearVelocity` (`self.Ball`) "None"))
  (set `self.CurrentVelocity` _returnvalue))

(fn `ApplyImpactImpulse`
  (params (OutgoingNormal :type "Vector Structure"))
  (`KismetSystemLibrary.PrintString` (`KismetStringLibrary.Conv_VectorToString` OutgoingNormal)))

(fn `UserConstructionScript`)