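; Paddle Blueprint that moves its Paddle component left and right from a tilt vector.
; UpdatePaddleLocation adds tilt X, scaled by a movement intensity, to the current relative X and clamps it to a symmetric limit around zero.
; It sets the location without sweeping, keeps Y and Z unchanged, and returns the new relative location for the Pawn.
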(fn `UpdatePaddleLocation`
  (params (TiltVector :type "Vector Structure"))
  (returns (PaddleRelativeLocation :type "Vector Structure"))
  (bind _paddlemovementlimit (`self.PaddleMovementLimit`))
  ;[1 1 1] Update paddle Location
  (`SceneComponent.K2_SetRelativeLocation` (`self.Paddle`) (`KismetMathLibrary.MakeVector` (`KismetMathLibrary.FClamp` (+ (* (.x TiltVector) (`self.PaddleMovementIntensity`)) (.x (`SceneComponent.RelativeLocation` (`self.Paddle`)))) (* -1.0 _paddlemovementlimit) _paddlemovementlimit) (.y (`SceneComponent.RelativeLocation` (`self.Paddle`))) (.z (`SceneComponent.RelativeLocation` (`self.Paddle`)))) false false)
  ;[1 1 1] Return Paddle Relative Location to Pawn
  (return (`SceneComponent.RelativeLocation` (`self.Paddle`))))

(fn `UserConstructionScript`)